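; Boss battle music actor that switches between pre-battle and battle tracks as the player moves through two trigger volumes.
; Entering PreBossBattle starts the lead-in track; entering BossBattle swaps it for the battle track, and leaving BossBattle swaps back.
; Leaving PreBossBattle stops the lead-in, with each FadeOut followed immediately by Deactivate.
; Overlaps respond only to BP_PlayerCharacter; the player reference cached at BeginPlay is otherwise unused.
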(event OnComponentBeginOverlap(PreBossBattle)
  (params (OverlappedComponent :type Primitive%20Component%20Object%20Reference) (OtherActor :type Actor%20Object%20Reference) (OtherComp :type Primitive%20Component%20Object%20Reference) (OtherBodyIndex :type Integer) (bFromSweep :type Boolean) (SweepResult :type Hit%20Result%20Structure%20%28by%20ref%29))
  (Utilities|Casting|CastToBP_PlayerCharacter OtherActor)
  (Components|Activation|Activate (Variables|Default|GetPreBossBattleMusic) false))

(event OnComponentBeginOverlap(BossBattle)
  (params (OverlappedComponent :type Primitive%20Component%20Object%20Reference) (OtherActor :type Actor%20Object%20Reference) (OtherComp :type Primitive%20Component%20Object%20Reference) (OtherBodyIndex :type Integer) (bFromSweep :type Boolean) (SweepResult :type Hit%20Result%20Structure%20%28by%20ref%29))
  (bind _prebossbattlemusic (Variables|Default|GetPreBossBattleMusic))
  (bind _bossbattlemusic (Variables|Default|GetBossBattleMusic))
  (Utilities|Casting|CastToBP_PlayerCharacter OtherActor)
  (Audio|Components|Audio|FadeOut _prebossbattlemusic 3.0 0.0 "Linear" :!class /Script/Engine.AudioComponent)
  (Components|Activation|Deactivate _prebossbattlemusic)
  (Components|Activation|Activate _bossbattlemusic false)
  (Audio|Components|Audio|FadeIn _bossbattlemusic 1.0 1.0 0.0 "Linear" :!class /Script/Engine.AudioComponent))

(event OnComponentEndOverlap(BossBattle)
  (params (OverlappedComponent :type Primitive%20Component%20Object%20Reference) (OtherActor :type Actor%20Object%20Reference) (OtherComp :type Primitive%20Component%20Object%20Reference) (OtherBodyIndex :type Integer))
  (bind _bossbattlemusic (Variables|Default|GetBossBattleMusic))
  (bind _prebossbattlemusic (Variables|Default|GetPreBossBattleMusic))
  (Utilities|Casting|CastToBP_PlayerCharacter OtherActor)
  (Audio|Components|Audio|FadeOut _bossbattlemusic 3.0 0.0 "Linear" :!class /Script/Engine.AudioComponent)
  (Components|Activation|Deactivate _bossbattlemusic)
  (Components|Activation|Activate _prebossbattlemusic false)
  (Audio|Components|Audio|FadeIn _prebossbattlemusic 1.0 1.0 0.0 "Linear" :!class /Script/Engine.AudioComponent))

(event OnComponentEndOverlap(PreBossBattle)
  (params (OverlappedComponent :type Primitive%20Component%20Object%20Reference) (OtherActor :type Actor%20Object%20Reference) (OtherComp :type Primitive%20Component%20Object%20Reference) (OtherBodyIndex :type Integer))
  (bind _prebossbattlemusic (Variables|Default|GetPreBossBattleMusic))
  (Utilities|Casting|CastToBP_PlayerCharacter OtherActor)
  (Audio|Components|Audio|FadeOut _prebossbattlemusic 3.0 0.0 "Linear" :!class /Script/Engine.AudioComponent)
  (Components|Activation|Deactivate _prebossbattlemusic))

(event EventBeginPlay
  (bind _asbp_player_character (Utilities|Casting|CastToBP_PlayerCharacter (Pawn|GetControlledPawn (Game|GetPlayerController 0))))
  (Variables|Default|SetPlayer _asbp_player_character))

(fn ConstructionScript)